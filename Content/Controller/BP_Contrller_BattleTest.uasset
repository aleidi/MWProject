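; Test player controller for battle target detection, with empty BeginPlay and Tick.
; Its SearchTargets event gets candidates from SearchSelectableTargets and prints their names on screen, but its only call in this graph is disconnected.
; A disconnected prototype checks recently rendered Characters against the camera's forward vector, widening the second angle limit as the horizontal angle grows, and prints the results.
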(event Custom|SearchTargets
  (bind _findtargets (Class|WMGameplayUtility|SearchSelectableTargets self (Utilities|Array|MakeArray 0)))
  (for _array_element _findtargets
    (Development|PrintString (Utilities|String|Append "findtarget : " (.Name (Utilities|Struct|BreakMWFoundActorInfo _array_element))) true false "(R=0.000000,G=0.660000,B=1.000000,A=1.000000)" 0.0)))

(event EventBeginPlay)

(event EventTick
  (params (DeltaSeconds :type Float%20%28single-precision%29)))

(event Input|KeyboardEvents|Z
  (params (Key :type Key%20Structure :default "None")))

(event Input|KeyboardEvents|AltZ
  (params (Key :type Key%20Structure :default "None")))

(fn ConstructionScript)