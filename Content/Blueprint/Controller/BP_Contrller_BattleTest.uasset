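; Test player controller for exercising the MW battle system's target selection and locking.
; On BeginPlay it binds to the target selected and locked events and prints each target's name.
; Debug keys switch, cancel, lock and unlock targets, or broadcast a hardcoded party update.
; Disconnected graphs hold target-search debug prints, including a camera view-angle test whose vertical limit widens with horizontal angle.
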(event Custom|SearchTargets
  (bind _findtargets (Class|WMGameplayUtility|SearchSelectableTargets self (Utilities|Array|MakeArray 0)))
  (for _array_element _findtargets
    (Development|PrintString (Utilities|String|Append "findtarget : " (.Name (Utilities|Struct|BreakMWFoundActorInfo _array_element))) true false "(R=0.000000,G=0.660000,B=1.000000,A=1.000000)" 0.0)))

(event Custom|OnTargetSelcted_Event
  (params (TargetInfo :type MW%20Found%20Actor%20Info%20Structure))
  (Development|PrintString (Utilities|String|Append "select target: " (.name TargetInfo))))

(event Custom|OnTargetLocked_Event
  (params (Target :type MW%20Found%20Actor%20Info%20Structure))
  (Development|PrintString (Utilities|String|Append "lock target: " (.name Target))))

(event EventBeginPlay
  (bind _returnvalue (Subsystems|GetMWBattleSystem))
  (EventDispatchers|BindEventtoOnTargetSelected _returnvalue (delegate Custom|OnTargetSelcted_Event))
  (EventDispatchers|AssignOnTargetLocked _returnvalue (delegate Custom|OnTargetLocked_Event)))

(event EventTick
  (params (DeltaSeconds :type Float%20%28single-precision%29)))

(event Input|KeyboardEvents|Z
  (params (Key :type Key%20Structure :default "None"))
  (:Pressed
    (Class|MWPlayerController|UnlockTarget)))

(event Input|KeyboardEvents|F
  (params (Key :type Key%20Structure :default "None"))
  (:Pressed
    (Default|CallOnPartyUpdate (Subsystems|GetMWBattleSystem) (Utilities|Struct|MakePartyInfo (Utilities|Array|MakeArray "TestG" "TestR")))))

(event Input|KeyboardEvents|E
  (params (Key :type Key%20Structure :default "None"))
  (:Pressed
    (Class|MWPlayerController|SwitchtoRight)))

(event Input|KeyboardEvents|SpaceBar
  (params (Key :type Key%20Structure :default "None"))
  (:Pressed
    (Class|MWPlayerController|LockTarget)))

(event Input|KeyboardEvents|Q
  (params (Key :type Key%20Structure :default "None"))
  (:Pressed
    (Class|MWPlayerController|SwitchtoLeft)))

(event Input|KeyboardEvents|AltQ
  (params (Key :type Key%20Structure :default "None"))
  (:Pressed
    (Class|MWPlayerController|CancelSelect)))

(fn ConstructionScript)